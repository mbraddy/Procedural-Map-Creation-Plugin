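; Procedural terrain actor that builds a collidable grid mesh from a heightmap and textures it using masks derived from a colored map.
; The construction script turns heightmap pixels into vertices, UVs, triangles and tangents for a procedural mesh section.
; BeginPlay creates color masks and a material, round-trips three masks through HDR files at hardcoded local paths, then assigns them as texture parameters and applies the material.
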(event `self.ReceiveBeginPlay`
  (bind _tempmat (`self.TempMat`))
  (bind _returnvalue (`self.CreateMasks` (`self.ColoredMap`) (`self.Colors`)))
  (set `self.OutputMasks` _returnvalue)
  (`KismetSystemLibrary.PrintText` "Masks Created" false)
  (bind _returnvalue_2 (`self.ApplyMasks` (`self.ColorTextures`) (`self.OutputMasks`) self))
  (set `self.TempMat` _returnvalue_2)
  (bind _returnvalue_3 (`self.GetMaskPackages`))
  (`KismetRenderingLibrary.ExportTexture2D` (`|GetArrayItem` _returnvalue_3) "C:\\Users\\mbraddy\\Documents\\Unreal Projects\\ProceduralMapTool\\Content\\ProceduralTextures\\" "COneMask.HDR")
  (`KismetRenderingLibrary.ExportTexture2D` (`|GetArrayItem` _returnvalue_3 1) "C:\\Users\\mbraddy\\Documents\\Unreal Projects\\ProceduralMapTool\\Content\\ProceduralTextures\\" "CTwoMask.HDR")
  (`KismetRenderingLibrary.ExportTexture2D` (`|GetArrayItem` _returnvalue_3 2) "C:\\Users\\mbraddy\\Documents\\Unreal Projects\\ProceduralMapTool\\Content\\ProceduralTextures\\" "CThreeMask.HDR")
  (`KismetRenderingLibrary.ExportTexture2D` "/Game/ProceduralTextures/ColorOneMask.COneMask" "C:\\Users\\mbraddy\\Documents\\Unreal Projects\\ProceduralMapTool\\Content\\ProceduralTextures\\" "COneMask.HDR")
  (`KismetRenderingLibrary.ExportTexture2D` "/Game/ProceduralTextures/ColorTwoMask.CTwoMask" "C:\\Users\\mbraddy\\Documents\\Unreal Projects\\ProceduralMapTool\\Content\\ProceduralTextures\\" "CTwoMask.HDR")
  (`KismetRenderingLibrary.ExportTexture2D` "/Game/ProceduralTextures/ColorThreeMask.CThreeMask" "C:\\Users\\mbraddy\\Documents\\Unreal Projects\\ProceduralMapTool\\Content\\ProceduralTextures\\" "CThreeMask.HDR")
  (bind _returnvalue_4 (`KismetRenderingLibrary.ImportFileAsTexture2D` "C:\\Users\\mbraddy\\Documents\\Unreal Projects\\ProceduralMapTool\\Content\\ProceduralTextures\\COneMask.HDR"))
  (set `self.MaskOne` _returnvalue_4)
  (bind _returnvalue_5 (`KismetRenderingLibrary.ImportFileAsTexture2D` "C:\\Users\\mbraddy\\Documents\\Unreal Projects\\ProceduralMapTool\\Content\\ProceduralTextures\\CTwoMask.HDR"))
  (set `self.MaskTwo` _returnvalue_5)
  (bind _returnvalue_6 (`KismetRenderingLibrary.ImportFileAsTexture2D` "C:\\Users\\mbraddy\\Documents\\Unreal Projects\\ProceduralMapTool\\Content\\ProceduralTextures\\CThreeMask.HDR"))
  (set `self.MaskThree` _returnvalue_6)
  (`MaterialInstanceDynamic.SetTextureParameterValue` _tempmat "ColorOneMask" (`self.MaskOne`))
  (`MaterialInstanceDynamic.SetTextureParameterValue` _tempmat "ColorTwoMask" (`self.MaskTwo`))
  (`MaterialInstanceDynamic.SetTextureParameterValue` _tempmat "ColorThreeMask" (`self.MaskThree`))
  (`PrimitiveComponent.SetMaterial` (`self.ProceduralMesh`) 0 (`self.TempMat`)))

(fn `UserConstructionScript`
  (bind _heightmap (`self.HeightMap`))
  (bind _heightmap_2 (`self.HeightMap`))
  (bind _returnvalue (`self.GetPixels` _heightmap))
  (set `self.Vertices` _returnvalue)
  (bind _returnvalue_2 (`self.GetUVs` _heightmap))
  (set `self.UVs` _returnvalue_2)
  (bind _triangles (`KismetProceduralMeshLibrary.CreateGridMeshTriangles` (`Texture2D.Blueprint_GetSizeX` _heightmap_2) (`Texture2D.Blueprint_GetSizeY` _heightmap_2)))
  (set `self.Triangles` _triangles)
  (bind (_normals _tangents) (`KismetProceduralMeshLibrary.CalculateTangentsForMesh` (`self.Vertices`) (`self.Triangles`) (`self.UVs`)))
  (set `self.Normals` _normals)
  (set `self.Tangents` _tangents)
  (`ProceduralMeshComponent.CreateMeshSection_LinearColor` :`self` (`self.ProceduralMesh`) :`Vertices` (`self.Vertices`) :`Triangles` (`self.Triangles`) :`Normals` (`self.Normals`) :`UV0` (`self.UVs`) :`Tangents` (`self.Tangents`) :`bCreateCollision` true))